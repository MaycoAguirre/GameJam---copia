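; Playable side-scroller character that moves along the X axis, jumps, fires projectiles and tracks health and coins.
; Enhanced Input drives movement, with control yaw flipped by the sign of acceleration, and spawns BP_proyectil behind a short cooldown.
; Coyote time opens a brief window after walking off a ledge in which jump launches the character upward.
; ObtenerVida and SumarPuntuacion events add to health and coin totals and print them.
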(event Input|EnhancedActionEvents|EnhancedInputActionIA_Desplazamiento
  (params (ActionValue :type Float%20%28double-precision%29) (ElapsedSeconds :type Float%20%28double-precision%29) (TriggeredSeconds :type Float%20%28double-precision%29) (InputAction :type Input%20Action%20Object%20Reference :default "/Game/BluePrints/Actores/PersonajeJugable/Inputs/IA_Desplazamiento.IA_Desplazamiento"))
  ;[1 1 1] Input de Movimiento
  (Pawn|Input|AddMovementInput "1.000000,0.000000,0.000000" ActionValue false)
  (Math|Float|CompareFloat (.x (Pawn|Components|CharacterMovement|GetCurrentAcceleration (Variables|Character|GetCharacterMovement))) 0.0
    (:>
      (Pawn|SetControlRotation (Pawn|GetController) (Math|Rotator|MakeRotator 0.0 0.0 0.0)))
    (:<
      (Pawn|SetControlRotation (Pawn|GetController) (Math|Rotator|MakeRotator 0.0 0.0 1.8e+02)))))

(event Input|EnhancedActionEvents|EnhancedInputActionIA_salto
  (params (ActionValue :type Boolean) (ElapsedSeconds :type Float%20%28double-precision%29) (TriggeredSeconds :type Float%20%28double-precision%29) (InputAction :type Input%20Action%20Object%20Reference :default "/Game/BluePrints/Actores/PersonajeJugable/Inputs/IA_salto.IA_salto"))
  ;[1 1 1] Agregar salto
  (:Started
    (Character|Jump)
    (if (Variables|Default|GetbCoyote%20Time?)
      (Character|LaunchCharacter "0.000000,0.000000,1000.000000" false true)))
  (:Completed
    (Character|StopJumping)))

(event Input|EnhancedActionEvents|EnhancedInputActionIA_AtaqueDistancia
  (params (ActionValue :type Boolean) (ElapsedSeconds :type Float%20%28double-precision%29) (TriggeredSeconds :type Float%20%28double-precision%29) (InputAction :type Input%20Action%20Object%20Reference :default "/Game/BluePrints/Actores/PersonajeJugable/Inputs/IA_AtaqueDistancia.IA_AtaqueDistancia"))
  ;[1 1 1] Input action de disparo de proyectil
  (:Started
    (if (not (Variables|Default|GetbDisparo?))
      (Variables|Default|SetbDisparo? true)
      (Game|SpawnActorfromClass "/Game/BluePrints/Actores/Proyectil/BP_proyectil.BP_proyectil_C" (Transformation|GetActorTransform) "Undefined" "MultiplyWithRoot" 0 1e+01 0)
      (Utilities|FlowControl|Delay 0.5)
      (Variables|Default|SetbDisparo? false))))

(event EventBeginPlay
  ;[1 1 1] Agregar Mapping Context
  (bind _asplayer_controller (Utilities|Casting|CastToPlayerController (Pawn|GetController)))
  (Input|AddMappingContext (PlayerController|LocalPlayerSubsystems|GetEnhancedInputLocalPlayerSubsystem _asplayer_controller) "/Game/BluePrints/Actores/PersonajeJugable/Inputs/MappingContext/IMC_Personaje.IMC_Personaje" 0 "(bIgnoreAllPressedKeysUntilRelease=True,bForceImmediately=False,bNotifyUserSettings=False)"))

(event EventObtenerVida
  (params (VidaExtra :type Float%20%28double-precision%29))
  (CallFunction|AñadirVida VidaExtra)
  (Development|PrintString (Utilities|String|ToString(Float) (Variables|Default|GetVidaActual))))

(event EventOnWalkingOffLedge
  (params (PreviousFloorImpactNormal :type Vector%20%28by%20ref%29 :default "0, 0, 0") (PreviousFloorContactNormal :type Vector%20%28by%20ref%29 :default "0, 0, 0") (PreviousLocation :type Vector%20%28by%20ref%29 :default "0, 0, 0") (TimeDelta :type Float%20%28single-precision%29))
  ;[1 1 1] Coyote time
  (Variables|Default|SetbCoyote%20Time? true)
  (Utilities|FlowControl|Delay 0.45)
  (Variables|Default|SetbCoyote%20Time? false))

(event EventSumarPuntuacion
  (params (SumarPunto :type Float%20%28double-precision%29))
  (CallFunction|SumarPuntos SumarPunto)
  (Development|PrintString (Utilities|String|ToString(Float) (Variables|Default|GetMonedasObtenidas))))

(fn ConstructionScript)

(fn AñadirVida
  (params (VidaAñadida :type Float%20%28double-precision%29))
  (Variables|Default|SetVidaActual (+ VidaAñadida (Variables|Default|GetVidaActual))))

(fn SumarPuntos
  (params (PuntoSumado :type Float%20%28double-precision%29))
  (Variables|Default|SetMonedasObtenidas (+ PuntoSumado (Variables|Default|GetMonedasObtenidas))))