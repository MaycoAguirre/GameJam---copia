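; Temporary platform actor that vanishes shortly after something overlaps its Box trigger, then reappears.
; Begin overlap disables the Box, waits briefly, hides the actor and turns off Cube collision, then restores visibility and both collisions after another delay.
; End overlap separately re-enables actor collision and unhides it after a delay.
; BeginPlay stores an unused initial position, and some disconnected debug and hide nodes remain.
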(event OnComponentBeginOverlap(Box)
  (params (OverlappedComponent :type Primitive%20Component%20Object%20Reference) (OtherActor :type Actor%20Object%20Reference) (OtherComp :type Primitive%20Component%20Object%20Reference) (OtherBodyIndex :type Integer) (bFromSweep :type Boolean) (SweepResult :type Hit%20Result%20Structure%20%28by%20ref%29))
  (Collision|SetCollisionEnabled (Variables|Default|GetBox) "NoCollision")
  (Utilities|FlowControl|Delay 1.0)
  (Collision|SetCollisionEnabled (Variables|Default|GetCube) "NoCollision")
  (Rendering|SetActorHiddenInGame true)
  (Utilities|FlowControl|Delay 2.0)
  (Rendering|SetActorHiddenInGame false)
  (Collision|SetCollisionEnabled (Variables|Default|GetCube) "QueryAndPhysics")
  (Collision|SetCollisionEnabled (Variables|Default|GetBox) "QueryAndPhysics"))

(event OnComponentEndOverlap(Box)
  (params (OverlappedComponent :type Primitive%20Component%20Object%20Reference) (OtherActor :type Actor%20Object%20Reference) (OtherComp :type Primitive%20Component%20Object%20Reference) (OtherBodyIndex :type Integer))
  (Utilities|FlowControl|Delay 2.0)
  (Collision|SetActorEnableCollision true)
  (Rendering|SetActorHiddenInGame false))

(event EventBeginPlay
  (Variables|Default|SetPosicionInicial (Transformation|GetActorLocation)))

(event Collision|EventActorBeginOverlap
  (params (OtherActor :type Actor%20Object%20Reference)))

(event EventTick
  (params (DeltaSeconds :type Float%20%28single-precision%29)))

(fn ConstructionScript)