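; BP_ENEMIGO is an enemy actor that moves along an InterpToMovement path between its origin and a configurable relative point.
; Box overlaps and EjecutarDaño share a path that passes damage through HacerDaño and messages it to the overlapped actor.
; Projectile hits arrive via BPIProyectil and reduce health, which starts at VidaMax, destroying the enemy at zero.
; PawnSensing only stores the seen pawn and prints an attack debug message.
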(event OnSeePawn(PawnSensing)
  (params (Pawn :type Pawn%20Object%20Reference))
  (bind _output_get (Variables|Default|SetPawn Pawn))
  (Development|PrintString (Utilities|String|Append "Atacaria a " (Utilities|GetDisplayName _output_get))))

(event OnComponentBeginOverlap(Box)
  (params (OverlappedComponent :type Primitive%20Component%20Object%20Reference) (OtherActor :type Actor%20Object%20Reference) (OtherComp :type Primitive%20Component%20Object%20Reference) (OtherBodyIndex :type Integer) (bFromSweep :type Boolean) (SweepResult :type Hit%20Result%20Structure%20%28by%20ref%29))
  (bind _dañofinal (CallFunction|HacerDaño (stale EventEjecutarDaño Daño)))
  (Class|BPIEnemigo|EjecutarDaño(Message) OtherActor _dañofinal)
  (Development|PrintString "daño al personaje"))

(event EventEjecutarDaño
  (params (Daño :type Float%20%28double-precision%29))
  (bind _dañofinal (CallFunction|HacerDaño Daño))
  (Class|BPIEnemigo|EjecutarDaño(Message) (stale OnComponentBeginOverlap(Box) OtherActor) _dañofinal)
  (Development|PrintString "daño al personaje"))

(event EventBeginPlay
  (Variables|Default|SetVidaActual (Variables|Default|GetVidaMax)))

(event EventBPIProyectil
  (params (DañoProyectil :type Float%20%28double-precision%29))
  (CallFunction|RecibirDaño DañoProyectil))

(fn ConstructionScript
  (Class|InterptoMovementComponent|AddControlPointPosition (Variables|Default|GetInterpToMovement) "0, 0, 0" true)
  (Class|InterptoMovementComponent|AddControlPointPosition (Variables|Default|GetInterpToMovement) (Variables|Default|GetPos) true))

(fn RecibirDaño
  (params (DañoRecibido :type Float%20%28double-precision%29))
  (bind _output_get (Variables|Default|SetVidaActual (- (Variables|Default|GetVidaActual) DañoRecibido)))
  (if (<= _output_get 0.0)
    (Actor|DestroyActor)))

(fn HacerDaño
  (params (DañoParametro :type Float%20%28double-precision%29))
  (bind _output_get (Variables|Default|SetDañoAPersonaje DañoParametro))
  (return _output_get))